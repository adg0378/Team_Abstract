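; Simulation manager that runs drone simulations, with a StartDemo event that rebuilds, loads and starts a test simulation.
; Start, end, restart, pause and resume events loop over all drones; pause and resume both call PauseDrone.
; Iso, EYE and front camera events forward the switch to the drone with the active camera.
; Progress is clamped and sent through CallSimPercentage as a float and rounded percentage text.
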(event `self.StartDemo`
  (bind _testonly (`self.TestOnly`))
  ; testing demo stuff
  (`self.UnloadSimulation`)
  (`self.CreateSimulation` _testonly)
  (`self.LoadSimulation` _testonly)
  (`self.SetSimulationDuration` 100000.0)
  (`self.StartSimulation`))

(event `self.StartSimulation`
  ; Simulation events
  (bind _returnvalue (`self.GetDrones`))
  (for _array_element _returnvalue
    (`DemoSimDrone.StartDroneMovement` _array_element)))

(event `self.SwapToIsoCam`
  ; Camera Swapping Stuff
  (bind _returnvalue (`self.GetCurrentActivateCamDrone`))
  (`BasicDrone.ActivateIsoCam` _returnvalue))

(event `self.SwapToEYECam`
  ; Camera Swapping Stuff
  (bind _returnvalue (`self.GetCurrentActivateCamDrone`))
  (`BasicDrone.ActivateEYECam` _returnvalue))

(event `self.EndSimulation`
  ; Simulation events
  (bind _returnvalue (`self.GetDrones`))
  (for _array_element _returnvalue
    (`DemoSimDrone.EndDroneMovement` _array_element)))

(event `self.SwapToFrontCam`
  ; Camera Swapping Stuff
  (bind _returnvalue (`self.GetCurrentActivateCamDrone`))
  (`BasicDrone.ActivateFrontCam` _returnvalue))

(event `self.RestartSimulation`
  ; Simulation events
  (bind _returnvalue (`self.GetDrones`))
  (for _array_element _returnvalue
    (`DemoSimDrone.RestartDrone` _array_element)))

(event `self.PauseSimulation`
  ; Simulation events
  (bind _returnvalue (`self.GetDrones`))
  (for _array_element _returnvalue
    (`DemoSimDrone.PauseDrone` _array_element)))

(event `self.ResumeSimulation`
  ; Simulation events
  (bind _returnvalue (`self.GetDrones`))
  (for _array_element _returnvalue
    (`DemoSimDrone.PauseDrone` _array_element)))

(event `self.GetSimProgressAsPercentage`
  (bind _returnvalue (`self.GetSimProgress`))
  (bind _returnvalue_2 (`KismetMathLibrary.FClamp` _returnvalue))
  (`self.SimPercentage` _returnvalue_2 (`KismetTextLibrary.Conv_TextToString` (`|FormatText` "{Percentage}%" (`KismetTextLibrary.Conv_DoubleToText` (`KismetMathLibrary.Conv_IntToDouble` (`KismetMathLibrary.Round` (* _returnvalue_2 100.0))) "HalfToEven")))))