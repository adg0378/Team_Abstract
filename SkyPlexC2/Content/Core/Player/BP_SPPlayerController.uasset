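; BP_SPPlayerController is the player controller that receives Enhanced Input for movement, camera control and selection-style actions.
; SetupEnhancedInput adds IMC_Default to the local player's input subsystem and registers it with user settings if needed.
; Each input action event, covering camera modes, mouse axes, cursor display, delete, multi-select and do-action start and completion, only forwards to a matching IA-prefixed function defined outside these graphs.
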(event `EnhancedInput|/Game/Core/Player/Input/IA_CameraPitch`
  (params (ActionValue :type "Float (double-precision)") (ElapsedSeconds :type "Float (double-precision)") (TriggeredSeconds :type "Float (double-precision)") (InputAction :type "InputAction Object Reference" :default "/Game/Core/Player/Input/IA_CameraPitch.IA_CameraPitch"))
  (:`Triggered`
    (`self.IACameraPitch` ActionValue)))

(event `EnhancedInput|/Game/Core/Player/Input/IA_FreeCamera`
  (params (ActionValue :type Boolean) (ElapsedSeconds :type "Float (double-precision)") (TriggeredSeconds :type "Float (double-precision)") (InputAction :type "InputAction Object Reference" :default "/Game/Core/Player/Input/IA_FreeCamera.IA_FreeCamera"))
  (:`Triggered`
    (`self.IAFreeCamera`)))

(event `EnhancedInput|/Game/Core/Player/Input/IA_ShowCursorInFirstPerson`
  (params (ActionValue :type Boolean) (ElapsedSeconds :type "Float (double-precision)") (TriggeredSeconds :type "Float (double-precision)") (InputAction :type "InputAction Object Reference" :default "/Game/Core/Player/Input/IA_ShowCursorInFirstPerson.IA_ShowCursorInFirstPerson"))
  (:`Triggered`
    (`self.IAShowCursorInFirstPerson`)))

(event `EnhancedInput|/Game/Core/Player/Input/IA_MouseX`
  (params (ActionValue :type "Float (double-precision)") (ElapsedSeconds :type "Float (double-precision)") (TriggeredSeconds :type "Float (double-precision)") (InputAction :type "InputAction Object Reference" :default "/Game/Core/Player/Input/IA_MouseX.IA_MouseX"))
  (:`Triggered`
    (`self.IAMouseX` ActionValue)))

(event `EnhancedInput|/Game/Core/Player/Input/IA_MouseY`
  (params (ActionValue :type "Float (double-precision)") (ElapsedSeconds :type "Float (double-precision)") (TriggeredSeconds :type "Float (double-precision)") (InputAction :type "InputAction Object Reference" :default "/Game/Core/Player/Input/IA_MouseY.IA_MouseY"))
  (:`Triggered`
    (`self.IAMouseY` ActionValue)))

(event `EnhancedInput|/Game/Core/Player/Input/IA_CameraZoomIn`
  (params (ActionValue :type Boolean) (ElapsedSeconds :type "Float (double-precision)") (TriggeredSeconds :type "Float (double-precision)") (InputAction :type "InputAction Object Reference" :default "/Game/Core/Player/Input/IA_CameraZoomIn.IA_CameraZoomIn"))
  (:`Triggered`
    (`self.IACameraZoomIn`)))

(event `EnhancedInput|/Game/Core/Player/Input/IA_CameraZoomOut`
  (params (ActionValue :type Boolean) (ElapsedSeconds :type "Float (double-precision)") (TriggeredSeconds :type "Float (double-precision)") (InputAction :type "InputAction Object Reference" :default "/Game/Core/Player/Input/IA_CameraZoomOut.IA_CameraZoomOut"))
  (:`Triggered`
    (`self.IACameraZoomOut`)))

(event `EnhancedInput|/Game/Core/Player/Input/IA_CameraOrbit`
  (params (ActionValue :type "Float (double-precision)") (ElapsedSeconds :type "Float (double-precision)") (TriggeredSeconds :type "Float (double-precision)") (InputAction :type "InputAction Object Reference" :default "/Game/Core/Player/Input/IA_CameraOrbit.IA_CameraOrbit"))
  (:`Triggered`
    (`self.IACameraOrbit` ActionValue)))

(event `EnhancedInput|/Game/Core/Player/Input/IA_Movement`
  (params (ActionValue :type "Vector Structure") (ElapsedSeconds :type "Float (double-precision)") (TriggeredSeconds :type "Float (double-precision)") (InputAction :type "InputAction Object Reference" :default "/Game/Core/Player/Input/IA_Movement.IA_Movement"))
  (:`Triggered`
    (`self.IAMovement` ActionValue)))

(event `EnhancedInput|/Game/Core/Player/Input/IA_SwapCamera1`
  (params (ActionValue :type Boolean) (ElapsedSeconds :type "Float (double-precision)") (TriggeredSeconds :type "Float (double-precision)") (InputAction :type "InputAction Object Reference" :default "/Game/Core/Player/Input/IA_SwapCamera1.IA_SwapCamera1"))
  (:`Triggered`
    (`self.IASwapCamera1`)))

(event `EnhancedInput|/Game/Core/Player/Input/IA_SwapCamera2`
  (params (ActionValue :type Boolean) (ElapsedSeconds :type "Float (double-precision)") (TriggeredSeconds :type "Float (double-precision)") (InputAction :type "InputAction Object Reference" :default "/Game/Core/Player/Input/IA_SwapCamera2.IA_SwapCamera2"))
  (:`Triggered`
    (`self.IASwapCamera2`)))

(event `EnhancedInput|/Game/Core/Player/Input/IA_SwapCamera3`
  (params (ActionValue :type Boolean) (ElapsedSeconds :type "Float (double-precision)") (TriggeredSeconds :type "Float (double-precision)") (InputAction :type "InputAction Object Reference" :default "/Game/Core/Player/Input/IA_SwapCamera3.IA_SwapCamera3"))
  (:`Triggered`
    (`self.IASwapCamera3`)))

(event `self.SetupEnhancedInput`
  (bind _returnvalue (subsystem `EnhancedInputLocalPlayerSubsystem`))
  (bind _returnvalue_2 (`EnhancedInputSubsystemInterface.GetUserSettings` _returnvalue))
  (`/Engine/EditorBlueprintResources/StandardMacros.IsValid` _returnvalue
    (:`Is Valid`
      (`EnhancedInputSubsystemInterface.AddMappingContext` _returnvalue "/Game/Core/Player/Input/IMC_Default.IMC_Default" 0 (struct))
      (if (not (`EnhancedInputUserSettings.IsMappingContextRegistered` _returnvalue_2 "/Game/Core/Player/Input/IMC_Default.IMC_Default"))
        (`EnhancedInputUserSettings.RegisterInputMappingContext` _returnvalue_2 "/Game/Core/Player/Input/IMC_Default.IMC_Default")))))

(event `EnhancedInput|/Game/Core/Player/Input/IA_Delete`
  (params (ActionValue :type Boolean) (ElapsedSeconds :type "Float (double-precision)") (TriggeredSeconds :type "Float (double-precision)") (InputAction :type "InputAction Object Reference" :default "/Game/Core/Player/Input/IA_Delete.IA_Delete"))
  (:`Triggered`
    (`self.IADelete`)))

(event `EnhancedInput|/Game/Core/Player/Input/IA_DoAction`
  (params (ActionValue :type Boolean) (ElapsedSeconds :type "Float (double-precision)") (TriggeredSeconds :type "Float (double-precision)") (InputAction :type "InputAction Object Reference" :default "/Game/Core/Player/Input/IA_DoAction.IA_DoAction"))
  (:`Started`
    (`self.IADoActionStarted`))
  (:`Completed`
    (`self.IADoActionCompleted`)))

(event `EnhancedInput|/Game/Core/Player/Input/IA_MultiSelect`
  (params (ActionValue :type Boolean) (ElapsedSeconds :type "Float (double-precision)") (TriggeredSeconds :type "Float (double-precision)") (InputAction :type "InputAction Object Reference" :default "/Game/Core/Player/Input/IA_MultiSelect.IA_MultiSelect"))
  (:`Triggered`
    (`self.IAMultipleSelect`)))

(fn `UserConstructionScript`)