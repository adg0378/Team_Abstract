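; BP_FAADOFObstacle is an FAA DOF obstacle actor placed on the Cesium globe, with a clickable, hoverable point widget.
; On BeginPlay it caches a base height from anchor height plus mesh bounds radius, then routes WB_ADSBPoint events to hover and click handlers.
; OnAnim moves the globe anchor vertically by scaling height above ground with the track value.
; ToggleCull shows or hides only the widget.
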(event `self.ReceiveBeginPlay`
  (`self.SetBaseZValue`)
  (bind _aswb_adsbpoint (cast `/Game/Objects/obstacles/WB_ADSBPoint` (`WidgetComponent.GetWidget` (`self.Widget`))))
  (add `/Game/Objects/obstacles/WB_ADSBPoint.OnClicked` _aswb_adsbpoint (delegate `OnObjectClicked`))
  (add `/Game/Objects/obstacles/WB_ADSBPoint.OnHovered` _aswb_adsbpoint (delegate `OnObjectHovered`))
  (add `/Game/Objects/obstacles/WB_ADSBPoint.OnHoverEnd` _aswb_adsbpoint (delegate `OnObjectHoverEnd`)))

(event `OnObjectHovered`
  (`self.OnHover` null))

(event `OnObjectClicked`
  (`self.OnClick` null))

(event `OnObjectHoverEnd`
  (`self.OnHoverEnd` null))

(event `self.ToggleCull`
  (params (IsCulled :type Boolean))
  (`SceneComponent.SetVisibility` (`self.Widget`) (not IsCulled) false))

(fn `OnAnim`
  (params (TrackVal :type "Float (double-precision)"))
  (bind _cesiumglobeanchor (`self.cesiumGlobeAnchor`))
  (`CesiumGlobeAnchorComponent.MoveToLongitudeLatitudeHeight` _cesiumglobeanchor (`KismetMathLibrary.MakeVector` (.x (`CesiumGlobeAnchorComponent.GetLongitudeLatitudeHeight` _cesiumglobeanchor)) (.y (`CesiumGlobeAnchorComponent.GetLongitudeLatitudeHeight` _cesiumglobeanchor)) (+ (* (`self.HeightAboveGroundLevelMeters`) TrackVal) (`self.BaseZVal`)))))

(fn `SetBaseZValue`
  (set `self.BaseZVal` (+ (/ (`.SphereRadius` (`KismetSystemLibrary.GetComponentBounds` (`self.staticMesh`))) 100.0) (.z (`CesiumGlobeAnchorComponent.GetLongitudeLatitudeHeight` (`self.cesiumGlobeAnchor`))))))

(fn `UserConstructionScript`)