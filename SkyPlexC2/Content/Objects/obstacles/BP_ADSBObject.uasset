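; BP_ADSBObject is an ADS-B obstacle object that shows an interactive point through a WB_ADSBPoint widget.
; On BeginPlay it binds to the widget's click, hover and hover-end events and relays them to OnClick, OnHover and OnHoverEnd.
; ToggleCull hides or shows the widget component according to the culled state, without propagating to children.
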(event `self.ReceiveBeginPlay`
  (bind _aswb_adsbpoint (cast `/Game/Objects/obstacles/WB_ADSBPoint` (`WidgetComponent.GetWidget` (`self.Widget`))))
  (add `/Game/Objects/obstacles/WB_ADSBPoint.OnClicked` _aswb_adsbpoint (delegate `OnButtonClicked`))
  (add `/Game/Objects/obstacles/WB_ADSBPoint.OnHovered` _aswb_adsbpoint (delegate `OnButtonHovered`))
  (add `/Game/Objects/obstacles/WB_ADSBPoint.OnHoverEnd` _aswb_adsbpoint (delegate `OnButtonHoverEnd`)))

(event `OnButtonClicked`
  (`self.OnClick` null))

(event `OnButtonHoverEnd`
  (`self.OnHoverEnd` null))

(event `OnButtonHovered`
  (`self.OnHover` null))

(event `self.ToggleCull`
  (params (IsCulled :type Boolean))
  (`SceneComponent.SetVisibility` (`self.Widget`) (not IsCulled) false))

(fn `UserConstructionScript`)