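; BP_SPSimWorldOrigin is an interest object that marks the sim world origin with a WB_SimWorldOrigin widget component.
; Widget click, hover and hover-end handlers forward to OnClick, OnHover and OnHoverEnd, while release does nothing.
; ToggleCull shows or hides the widget component and its children.
; The code that binds the handlers to the widget is disconnected, so this graph never hooks them up.
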(event `CustomEvent`)

(event `OnWidgetClicked`
  (`self.OnClick` null))

(event `OnWidgetHovered`
  (`self.OnHover` null))

(event `OnWidgetHoverEnd`
  (`self.OnHoverEnd` null))

(event `OnWidgetReleased`)

(event `self.ToggleCull`
  (params (IsCulled :type Boolean) (FromFlyTo :type Boolean))
  (`SceneComponent.SetVisibility` (`self.Widget`) (not IsCulled) true))

(fn `UserConstructionScript`)