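; BP_Polygon is a geometry actor that shows an area as a highlight on a Cesium 3D tileset, an outline, or both.
; Highlighting spawns or updates a CesiumCartographicPolygon from actor locations and registers it with the tileset's polygon raster overlay tagged "Blue", refreshing on each change.
; Outlining spawns a BP_InterestLines through the same points, passing that tag.
; The construction script finds a tileset if none is set.
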(event `self.Highlight`
  (`self.DoHighlight`)
  (`self.DoOutline`))

(event `self.UnHighlight`
  (`self.DoUnhighlight`)
  (`self.DoUnoutline`))

(event `self.HighlightOnly`
  (params (IsHighlighted :type Boolean))
  (if IsHighlighted
    (`self.DoHighlight`)
    (else
      (`self.DoUnhighlight`))))

(event `self.OutlineOnly`
  (params (IsOutlined :type Boolean))
  (if IsOutlined
    (`self.DoOutline`)
    (else
      (`self.DoUnoutline`))))

(fn `DoHighlight`
  (bind _cartographicpoly (`self.CartographicPoly`))
  (bind _cartographicpoly_2 (`self.CartographicPoly`))
  (bind _outactorlocations (`self.GetActorLocations`))
  (`/Engine/EditorBlueprintResources/StandardMacros.IsValid` _cartographicpoly_2
    (:`Is Valid`
      (`SplineComponent.SetSplinePoints` (`CesiumCartographicPolygon.Polygon` _cartographicpoly_2) _outactorlocations "World" true)
      (bind _cesiumpolygonrasteroverlay (`self.GetPolygonRasterOverlay`))
      (`CesiumRasterOverlay.Refresh` _cesiumpolygonrasteroverlay))
    (:`Is Not Valid`
      (bind _returnvalue (`|SpawnActorFromClass` "/Script/CesiumRuntime.CesiumCartographicPolygon" (`KismetMathLibrary.MakeTransform` (`KismetMathLibrary.GetVectorArrayAverage` _outactorlocations)) "Undefined" "MultiplyWithRoot" self null))
      (bind _output_get (set `self.CartographicPoly` _returnvalue))
      (`self.K2_AttachToActor` _output_get self "None" "KeepWorld" "KeepWorld" "KeepWorld" true)
      (`SplineComponent.SetSplinePoints` (`CesiumCartographicPolygon.Polygon` _cartographicpoly) _outactorlocations "World" true)
      (bind _cesiumpolygonrasteroverlay_2 (`self.GetPolygonRasterOverlay`))
      (`KismetArrayLibrary.Array_AddUnique` (`CesiumPolygonRasterOverlay.Polygons` _cesiumpolygonrasteroverlay_2) (`|ConvertAsset` _cartographicpoly))
      (`CesiumRasterOverlay.Refresh` _cesiumpolygonrasteroverlay_2))))

(fn `DoOutline`
  (bind _interestlines (`self.InterestLines`))
  (`/Engine/EditorBlueprintResources/StandardMacros.IsValid` _interestlines
    (:`Is Valid`
      (`InterestLines.DestroyInterestLines` _interestlines))
    (:`Is Not Valid`
      _))
  (bind _outactorlocations (`self.GetActorLocations`))
  (bind _returnvalue (`|SpawnActorFromClass` "/Game/Objects/Geometry/BP_InterestLines.BP_InterestLines_C" (`KismetMathLibrary.MakeTransform` (`|GetArrayItem` _outactorlocations)) "Undefined" "MultiplyWithRoot" self null))
  (bind _output_get (set `self.InterestLines` _returnvalue))
  (`InterestLines.DrawLinesViaActorLocations` _output_get _outactorlocations (`KismetStringLibrary.Conv_NameToString` (`self.PolygonRasterOverlayHasTag`))))

(fn `DoUnhighlight`
  (bind _cesiumpolygonrasteroverlay (`self.GetPolygonRasterOverlay`))
  (`KismetArrayLibrary.Array_RemoveItem` (`CesiumPolygonRasterOverlay.Polygons` _cesiumpolygonrasteroverlay) (`|ConvertAsset` (`self.CartographicPoly`)))
  (`CesiumRasterOverlay.Refresh` _cesiumpolygonrasteroverlay)
  (`self.K2_DestroyActor` (`self.CartographicPoly`)))

(fn `DoUnoutline`
  (`InterestLines.DestroyInterestLines` (`self.InterestLines`)))

(fn `GetPolygonRasterOverlay`
  (returns (CesiumPolygonRasterOverlay :type "CesiumPolygonRasterOverlay Object Reference"))
  (for _array_element (`self.K2_GetComponentsByClass` (`self.Tileset`) "/Script/CesiumRuntime.CesiumPolygonRasterOverlay")
    (if (`ActorComponent.ComponentHasTag` _array_element (`self.PolygonRasterOverlayHasTag`))
      (return _array_element)))
  (return _array_element))

(fn `PolygonRasterOverlayHasTag`
  (returns (Tag :type Name))
  (return "Blue"))

(fn `UserConstructionScript`
  (`self.Tileset`
    (:`then`)
    (:`else`
      (bind _returnvalue (`GameplayStatics.GetActorOfClass` "/Script/CesiumRuntime.Cesium3DTileset"))
      (set `self.Tileset` _returnvalue))))