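; BP_InterestLines draws colored interest lines, such as areas of interest or geofences, on the ground along a spline using decals.
; SpawnInterestLines first snaps each spline point to the surface with vertical traces (commented as unused, though still wired).
; It then adds downward-projected decals at fixed distances along the spline, following its yaw and roll.
; SetLineColorViaTag picks the blue, red or default decal material.
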(event `self.SpawnInterestLines`
  (bind _drawingspline (`self.DrawingSpline`))
  (bind _drawingspline_2 (`self.DrawingSpline`))
  (`|ExecutionSequence`
    (:`then_0`
      (for _index (range (`SplineComponent.GetNumberOfSplinePoints` _drawingspline_2))
        (bind (_returnvalue_x _returnvalue_y _returnvalue_z) (`KismetMathLibrary.BreakVector` (`SplineComponent.GetLocationAtSplinePoint` _drawingspline_2 _index "World")))
        (bind (_returnvalue_x_2 _returnvalue_y_2 _returnvalue_z_2) (`KismetMathLibrary.BreakVector` (`SplineComponent.GetLocationAtSplinePoint` _drawingspline_2 _index "World")))
        (bind (_outhit _returnvalue) (`KismetSystemLibrary.LineTraceSingle` (`KismetMathLibrary.MakeVector` _returnvalue_x _returnvalue_y (+ _returnvalue_z 1000.0)) (`KismetMathLibrary.MakeVector` _returnvalue_x_2 _returnvalue_y_2 (- _returnvalue_z_2 1000.0)) "TraceTypeQuery3" false (`self.ActorsNotToBeDrawnOn`)))
        (if _returnvalue
          (`SplineComponent.SetLocationAtSplinePoint` (`self.DrawingSpline`) _index (`.Location` (`GameplayStatics.BreakHitResult` _outhit)) "World" true))))
    (:`then_1`
      (for _index_2 (range (+ (`KismetMathLibrary.FTrunc` (/ (`SplineComponent.GetSplineLength` _drawingspline) 256.0)) 1))
        (bind _returnvalue_2 (`AddComponent|NODE_AddDecalComponent-0` :`RelativeTransform` (`KismetMathLibrary.MakeTransform` (0.0 0.0 0.0) (struct :`Pitch` 90.0))))
        (bind _returnvalue_3 (`KismetMathLibrary.Conv_IntToDouble` (* _index_2 256)))
        (bind (_returnvalue_roll _returnvalue_pitch _returnvalue_yaw) (`KismetMathLibrary.BreakRotator` (`SplineComponent.GetRotationAtDistanceAlongSpline` _drawingspline _returnvalue_3 "World")))
        (`SceneComponent.K2_SetWorldLocationAndRotation` _returnvalue_2 (`SplineComponent.GetLocationAtDistanceAlongSpline` _drawingspline _returnvalue_3 "World") (`KismetMathLibrary.MakeRotator` (- _returnvalue_roll 90.0) 90.0 _returnvalue_yaw) false false)
        (`DecalComponent.SetDecalMaterial` _returnvalue_2 (`self.LineDecal`))))))

(event `self.SetLineColorViaTag`
  (params (tag :type String))
  (if (== tag "Blue")
    (set `self.LineDecal` (`self.AOIDecal`))
    (elif (== tag "Red")
      (set `self.LineDecal` (`self.GeoFenceDecal`))
      (else
        (set `self.LineDecal` "/Game/Materials/M_InterestSplineDecalBase.M_InterestSplineDecalBase")))))

(fn `UserConstructionScript`)