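; Demo simulation drone actor that flies along the spline of a referenced drone track.
; A timeline, rate-scaled by Duration and begun at a start offset, maps its alpha to distance along the spline and sets the actor transform without sweep, sampled in local space.
; Custom events start, pause, resume from saved progress, restart or end the flight, with ending resetting progress to zero.
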(event `self.StartDroneMovement`
  (bind _drone_movement (`self.Drone Movement`))
  ; Movement Logic
  (bind _returnvalue (`self.GetDuration`))
  (`TimelineComponent.SetPlayRate` _drone_movement (/ 1.0 _returnvalue))
  (bind _returnvalue_2 (`self.GetStartOffset`))
  (`TimelineComponent.SetNewTime` _drone_movement _returnvalue_2)
  (bind (_direction _alpha) (`Timeline|Drone Movement` :!label _label)
    (:`Update`
      (bind _output_get (set `self.Alpha` _alpha))
      (`self.SetProgress` _output_get)
      (bind _returnvalue_3 (`self.GetDroneTrack`))
      (bind _splinetrack (`DroneTrack.SplineTrack` _returnvalue_3))
      (`self.K2_SetActorTransform` (`SplineComponent.GetTransformAtDistanceAlongSpline` _splinetrack (`KismetMathLibrary.Lerp` 0.0 (`SplineComponent.GetSplineLength` _splinetrack) (`self.Alpha`)) "Local" false)))))

(event `self.ResumeDrone`
  ; Movement Logic
  (bind _returnvalue (`self.GetProgress`))
  (`TimelineComponent.SetNewTime` (`self.Drone Movement`) _returnvalue)
  (goto _label))

(event `self.RestartDrone`
  ; Movement Logic
  (goto _label :!via `PlayFromStart`))

(event `self.EndDroneMovement`
  ; Movement Logic
  (`self.SetProgress` 0.0)
  (goto _label :!via `Stop`))

(event `self.PauseDrone`
  ; Movement Logic
  (goto _label :!via `Stop`))

(fn `UserConstructionScript`)