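; BP_CCSimDrone is a simulation drone object represented by a WB_DronePoint marker on its Widget component.
; On BeginPlay it binds the marker's hover, hover-end and click events, forwarding them to the drone's OnHover, OnHoverEnd and OnClick handlers.
; The marker title comes from the interaction box title and updates whenever that title changes.
; ToggleCull hides or shows the widget component according to the cull state.
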(event `self.ReceiveBeginPlay`
  (bind _aswb_drone_point (cast `/Game/Objects/drone/WB_DronePoint` (`WidgetComponent.GetWidget` (`self.Widget`))))
  (add `/Game/Objects/drone/WB_DronePoint.OnHovered` _aswb_drone_point (delegate `OnObjectHovered`))
  (add `/Game/Objects/drone/WB_DronePoint.OnHoverEnd` _aswb_drone_point (delegate `OnObjectHoverEnd`))
  (add `/Game/Objects/drone/WB_DronePoint.OnClicked` _aswb_drone_point (delegate `OnObjectClicked`))
  (bind _outtitle (`InteractionBoxProvider.GetInteractionBoxTitle`))
  (`/Game/Objects/drone/WB_DronePoint.UpdateTitleText` _aswb_drone_point _outtitle))

(event `OnObjectHoverEnd`
  (`self.OnHoverEnd` null))

(event `OnObjectHovered`
  (`self.OnHover` null))

(event `OnObjectClicked`
  (`self.OnClick` null))

(event `self.ToggleCull`
  (params (IsCulled :type Boolean) (FromFlyTo :type Boolean))
  (`SceneComponent.SetVisibility` (`self.Widget`) (not IsCulled) false))

(event `self.OnInteractionBoxTitleChanged`
  (params (NewTitle :type "Text (by ref)"))
  (bind _aswb_drone_point (cast `/Game/Objects/drone/WB_DronePoint` (`WidgetComponent.GetWidget` (`self.Widget`))))
  (`/Game/Objects/drone/WB_DronePoint.UpdateTitleText` _aswb_drone_point NewTitle))

(fn `UserConstructionScript`)